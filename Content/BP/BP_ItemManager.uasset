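; BP_ItemManager manages item spawning, transformation and placement for two players, creating Player 2 copies of the placed BP_Item actors.
; It caches DT_Items rows, draws random starting items from self-parented base rows and builds a desired-item list from Player 1's items.
; A dropped item shifts to a neighbouring row by its Basic/Rough/Fine value and WantToMakeFine, then updates meshes and teleports.
; Destroy-and-respawn and round-completion logic are left unwired.
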(event Custom|Destroy_Item
  (params (player_Index :type Integer))
  (switch int player_Index
    (:0
      (CallFunction|ChangeItemMoveItem false))
    (:1
      (CallFunction|ChangeItemMoveItem false 1))))

(event Custom|SetNewPosition_on_Init
  ;[0.15 0.15 0.15 0.5] set pos on init
  (CallFunction|SetNewPositionInitilisation))

(event Custom|FindItem_toSpawn
  (params (player_Index :type Integer))
  ;[0.15 0.15 0.15 0.5] Find next item after dropping it, and spawn it
  (switch int player_Index
    (:Default
      (CallFunction|ChangeInputedItem (Variables|Default|GetCurrentItems_P1) (Variables|Default|GetDroppedItem_P1) player_Index :!label _label)
      (CallFunction|ChangeItemMoveItem false player_Index))
    (:0
      (goto _label))
    (:1
      (CallFunction|ChangeInputedItem (Variables|Default|GetCurrentItems_P2) (Variables|Default|GetDroppedItem_P2) player_Index)
      (CallFunction|ChangeItemMoveItem false player_Index))))

(event Custom|SpawnRandomItem%281%29
  (bind _bp_item_ref_player1 (Variables|Default|GetBP_Item_Ref_Player1))
  (bind _returnvalue (Utilities|Array|Length _bp_item_ref_player1))
  ;[0.3417 0.4671 0.5573] spawn initial item (at random)
  (if (<= _returnvalue 1)
    (CallFunction|GetRandItemfromInitArrayandSetCurrentItem)
    (CallFunction|ChangeItemMoveItem true)
    (else
      (for _index (range 0 _returnvalue)
        (CallFunction|GetRandItemfromInitArrayandSetCurrentItem _index))
      (CallFunction|ChangeItemMoveItem false)))
  (CallFunction|CreateListOfDesiredItems))

(event Custom|Init_InitialSpawnableItems
  ;[0.195 0.5104 0.1914 0.5] Initialisation
  ;;[0.2462 0.09084 0.1912] Create list of base (1) items
  (bind _array_element (Utilities|Array|ForEachLoopwithBreak (Variables|Default|GetDT_Array))
    (:LoopBody
      (bind _returnvalue (Utilities|GetDataTableRow "/Game/Structs/DT_Items.DT_Items" _array_element)
        (:then
          (if (Utilities|Enum|Equal(Enum) (.parent_object _returnvalue) (.object_name _returnvalue))
            (Utilities|Array|Add (Variables|Default|GetInitialItemsToSpawn) _array_element)))))))

(event Custom|ChangeItem_MoveItem
  (params (All_Items? :type Boolean) (player_Index :type Integer))
  ;[0 0.1172 0.526 0.5] Change item mesh + spawn at location
  (CallFunction|SetNewStaticMesh)
  (if All_Items?
    (CallFunction|SetNewPositionInitilisation)
    (else
      (CallFunction|SetNewPosforSingleItemSinglePlayer player_Index))))

(event Custom|SpawnAnyItem
  ;[0.3342 0.4569 0.5469] spawn any initial item of big list
  (if (<= (Utilities|Array|LastIndex (Variables|Default|GetCurrentItems_P1)) 0)
    (CallFunction|GetRandItemfromFULLArrayandSetCurrentItem)
    (CallFunction|ChangeItemMoveItem false)
    (else
      (for (_ _array_index) (Variables|Default|GetCurrentItems_P1)
        (CallFunction|GetRandItemfromFULLArrayandSetCurrentItem _array_index))
      (CallFunction|ChangeItemMoveItem false)))
  (CallFunction|CreateListOfDesiredItems))

(event Custom|Set_DroppedItem
  (params (DroppedItem :type STRUCT%20Items%20Structure))
  ;[1 0.8626 0 0.5] Set dropped item
  (Variables|Default|SetDroppedItem_P1 DroppedItem))

(event Custom|SetValue_WantToMakeFine?
  (params (WantToMakeFine? :type Boolean))
  ;[1 0.924 0 0.5] Set val of "WantToMakeFine?"
  (Variables|Default|SetWantToMakeFine? WantToMakeFine?))

(event Custom|WhatItemIsThis?
  (params (ItemID :type Integer) (PlayerID :type Integer))
  ;[0.15 0.15 0.15 0.5] what item is this?
  (for (_array_element _array_index) (Variables|Default|GetDT_Array)
    (Utilities|GetDataTableRow "/Game/Structs/DT_Items.DT_Items" _array_element
      (:then
        (if (== _array_index ItemID)
          (bind _returnvalue (Utilities|GetDataTableRow "/Game/Structs/DT_Items.DT_Items" _array_element)
            (:then
              (switch int PlayerID
                (:0
                  (Variables|Default|SetDroppedItem_P1 _returnvalue))
                (:1
                  (Variables|Default|SetDroppedItem_P2 _returnvalue))))))))))

(event EventBeginPlay
  ;[0.195 0.5104 0.1914 0.5] Initialisation
  ;;[0.6042 0.2234 0.4732 0.5] initialise DT array
  (bind _outrownames (DataTable|GetDataTableRowNames "/Game/Structs/DT_Items.DT_Items"))
  (for (_array_element _array_index) _outrownames
    (Utilities|Array|SetArrayElem (Variables|Default|GetDT_Array) _array_index _array_element true))
  ;;[0.1042 0.3001 0.5885 0.5] find and create Bp_Items
  (bind _outactors (Actor|GetAllActorsOfClass "/Game/BP/BP_Item.BP_Item_C"))
  (bind _output_get (Variables|Default|SetBP_Item_Ref_Player1 _outactors))
  (CallFunction|CreateCopiesforP2 _output_get)
  ;;[0.15 0.02734 0.02734 0.5] BP_MoveObjectHere Ref
  (for _array_element_2 (Variables|Default|GetBP_MoveObjectHere_Ref)
    (Utilities|Array|Add (Variables|Default|GetMoveItemHere) (Transformation|GetActorTransform _array_element_2)))
  (CallFunction|InitInitialSpawnableItems))

(fn ConstructionScript)

(fn SetNewPositionInitilisation
  ;[0.15 0.15 0.15 0.5] move to pos 1
  (for _array_element (Variables|Default|GetBP_Item_Ref_Player1)
    (Transformation|SetActorTransform _array_element (Utilities|Array|Get(acopy) (Variables|Default|GetMoveItemHere)) false true))
  ;[0.15 0.15 0.15 0.5] move to pos 2
  (for _array_element_2 (Variables|Default|GetBP_Item_Ref_Player2)
    (Transformation|SetActorTransform _array_element_2 (Utilities|Array|Get(acopy) (Variables|Default|GetMoveItemHere) 1) false true))
  (return))

(fn SetNewStaticMesh
  (bind _currentitems_p2 (Variables|Default|GetCurrentItems_P2))
  (for (_array_element _array_index) (Variables|Default|GetBP_Item_Ref_Player1)
    (Default|SetItemData _array_element (Utilities|Array|Get(acopy) (Variables|Default|GetCurrentItems_P1) _array_index))
    (Default|SetStaticMesh _array_element))
  (for (_array_element_2 _array_index_2) (Variables|Default|GetBP_Item_Ref_Player2)
    (Components|StaticMesh|SetStaticMesh (Variables|/Game/BP/BP_Item.BP_Item_C|GetStaticMesh _array_element_2) (.staticmesh_reference (Utilities|Array|Get(acopy) _currentitems_p2 _array_index_2)))
    (Default|SetItemData _array_element_2 (Utilities|Array|Get(acopy) _currentitems_p2 _array_index_2)))
  (return))

(fn PlayRoughSFX
  (params (player_Index :type Integer)))

(fn PlayFineSFX
  (params (playerIndex :type Integer))
  (return))

(fn FindInitialParentItemDroppedItem
  (bind _array_element (Utilities|Array|ForEachLoopwithBreak (Variables|Default|GetDT_Array))
    (:LoopBody
      (bind _returnvalue (Utilities|GetDataTableRow "/Game/Structs/DT_Items.DT_Items" _array_element)
        (:then
          (if (Utilities|Enum|Equal(Enum) (.object_name _returnvalue) (.parent_object (Variables|Default|GetDroppedItem_P1)))
            (bind _itemindex (CallFunction|FindDroppedItemIndexinCurrentItemsP1))
            (return _array_element _itemindex (.object_name _returnvalue))))))))

(fn GetRandItemfromInitArrayandSetCurrentItem
  (params (IndexToSet :type Integer))
  (bind _returnvalue (Utilities|GetDataTableRow "/Game/Structs/DT_Items.DT_Items" (Utilities|Array|Get(acopy) (Variables|Default|GetInitialItemsToSpawn) (Math|Random|RandomInteger (- (Utilities|Array|LastIndex (Variables|Default|GetInitialItemsToSpawn)) 1))))
    (:then
      (Utilities|Array|SetArrayElem (Variables|Default|GetCurrentItems_P1) IndexToSet _returnvalue true)
      (Utilities|Array|SetArrayElem (Variables|Default|GetCurrentItems_P2) IndexToSet _returnvalue true)
      (return))))

(fn CreateCopiesforP2
  (params (Array :type Array%20of%20BP%20Item%20Object%20References))
  (for (_array_element _array_index) Array
    (bind _returnvalue (Game|SpawnActorfromClass "/Game/BP/BP_Item.BP_Item_C" (Math|Transform|MakeTransform (Math|Vector|MakeVector (* (+ (.x (.location (Transformation|GetActorTransform _array_element))) 1e+02) _array_index) (.y (.location (Transformation|GetActorTransform _array_element))) (.z (.location (Transformation|GetActorTransform _array_element)))) "0, 0, 0" "1.000000,1.000000,1.000000") "AlwaysSpawn" "MultiplyWithRoot" 0 0))
    (Utilities|Array|SetArrayElem (Variables|Default|GetBP_Item_Ref_Player2) _array_index _returnvalue true)
    (Variables|/Game/BP/BP_Item.BP_Item_C|SetPlayerIndex _returnvalue 1))
  (return))

(fn GetRandItemfromFULLArrayandSetCurrentItem
  (params (Index :type Integer))
  (Utilities|GetDataTableRow "/Game/Structs/DT_Items.DT_Items" (Utilities|Array|Get(acopy) (Variables|Default|GetDT_Array) (Math|Random|RandomInteger (Utilities|Array|LastIndex (Variables|Default|GetDT_Array))))
    (:then
      (Utilities|Array|SetArrayElem :TargetArray (Variables|Default|GetCurrentItems_P1) :Index Index :bSizeToFit true)
      (return))))

(fn FindDroppedItemIndexinCurrentItems
  (params (CurrentItems :type Array%20of%20STRUCT%20Items%20Structures) (DroppedItems :type STRUCT%20Items%20Structure))
  (bind (_array_element _array_index) (Utilities|Array|ForEachLoopwithBreak CurrentItems :!label _label)
    (:LoopBody
      (if (== (.staticmesh_reference _array_element) (.staticmesh_reference DroppedItems))
        (goto _label Break)))
    (:Completed
      (return _array_index))))

(fn SetNewIteminCurrentItems
  (params (Item :type STRUCT%20Items%20Structure%20%28by%20ref%29) (TargetArray :type Array%20of%20STRUCT%20Items%20Structures))
  (bind _arrayindex (CallFunction|FindDroppedItemIndexinCurrentItems))
  (Utilities|Array|SetArrayElem TargetArray _arrayindex Item))

(fn ChangeInputedItem
  (params (CurrentItems :type Array%20of%20STRUCT%20Items%20Structures) (DroppedItem :type STRUCT%20Items%20Structure) (player_Index :type Integer))
  (bind (_itemid _parent_object _object_name) (Utilities|Struct|BreakSTRUCT_Items DroppedItem))
  (bind _array_element (Utilities|Array|ForEachLoopwithBreak (Variables|Default|GetDT_Array))
    (:LoopBody
      (bind _returnvalue (Utilities|GetDataTableRow "/Game/Structs/DT_Items.DT_Items" _array_element)
        (:then
          ;[0.15 0.15 0.15 0.5] is object == row parent?
          (if (Utilities|Enum|Equal(Enum) (.parent_object _returnvalue) _parent_object)
            ;[0.15 0.15 0.15 0.5] Is object name ==?
            (if (Utilities|Enum|Equal(Enum) (.object_name _returnvalue) _object_name)
              ;[0.15 0.15 0.15 0.5] value of machine
              (if (Variables|Default|GetWantToMakeFine?)
                (switch Utilities|FlowControl|Switch|SwitchonENUM_ItemStates (.internal_value _returnvalue)
                  (:NewEnumerator0
                    (CallFunction|DestroyItem player_Index))
                  (:NewEnumerator1
                    (bind _returnvalue_2 (Utilities|GetDataTableRow "/Game/Structs/DT_Items.DT_Items" (Utilities|Array|Get(acopy) (Variables|Default|GetDT_Array) (- _itemid 1)))
                      (:then
                        (CallFunction|SetNewIteminCurrentItems _returnvalue_2 CurrentItems))))
                  (:NewEnumerator2
                    (bind _returnvalue_3 (Utilities|GetDataTableRow "/Game/Structs/DT_Items.DT_Items" (Utilities|Array|Get(acopy) (Variables|Default|GetDT_Array) (- _itemid 1)))
                      (:then
                        (CallFunction|SetNewIteminCurrentItems _returnvalue_3 CurrentItems)))))
                (else
                  (switch Utilities|FlowControl|Switch|SwitchonENUM_ItemStates (.internal_value _returnvalue)
                    (:NewEnumerator0
                      (bind _returnvalue_4 (Utilities|GetDataTableRow "/Game/Structs/DT_Items.DT_Items" (Utilities|Array|Get(acopy) (Variables|Default|GetDT_Array) (+ _itemid 2)))
                        (:then
                          (CallFunction|SetNewIteminCurrentItems _returnvalue_4 CurrentItems))))
                    (:NewEnumerator1
                      (CallFunction|DestroyItem player_Index))
                    (:NewEnumerator2
                      (bind _returnvalue_5 (Utilities|GetDataTableRow "/Game/Structs/DT_Items.DT_Items" (Utilities|Array|Get(acopy) (Variables|Default|GetDT_Array) (- _itemid 1)))
                        (:then
                          (CallFunction|SetNewIteminCurrentItems _returnvalue_5 CurrentItems))))))))))))
    (:Completed
      (return))))

(fn SetNewPosforSingleItemSinglePlayer
  (params (player_Index :type Integer))
  (switch int player_Index
    (:Default
      (for (_array_element _array_index) (Variables|Default|GetCurrentItems_P1) :!label _label
        (if (== (.staticmesh_reference _array_element) (.staticmesh_reference (Variables|Default|GetDroppedItem_P1)))
          (Transformation|SetActorTransform (Utilities|Array|Get(acopy) (Variables|Default|GetBP_Item_Ref_Player1) _array_index) (Utilities|Array|Get(acopy) (Variables|Default|GetMoveItemHere)) false true)
          (return))))
    (:0
      (goto _label))
    (:1
      (for (_array_element_2 _array_index_2) (Variables|Default|GetCurrentItems_P2)
        (if (== (.staticmesh_reference _array_element_2) (.staticmesh_reference (Variables|Default|GetDroppedItem_P2)))
          (Transformation|SetActorTransform (Utilities|Array|Get(acopy) (Variables|Default|GetBP_Item_Ref_Player2) _array_index_2) (Utilities|Array|Get(acopy) (Variables|Default|GetMoveItemHere) 1) false true)
          (return))))))

(fn FindDroppedItemIndexinCurrentItemsP1
  (bind _droppeditem_p1 (Variables|Default|GetDroppedItem_P1))
  (for (_array_element _array_index) (Variables|Default|GetCurrentItems_P1)
    (if (== (.itemid _array_element) (.itemid _droppeditem_p1))
      (if (Utilities|Enum|Equal(Enum) (Utilities|String|ToString(Text) (.parent_object _array_element)) (Utilities|String|ToString(Text) (.parent_object _droppeditem_p1)))
        (return _array_index)
        (else
          (return -1))))))

(fn FindDroppedItemIndexinCurrentItemsP2
  (for (_array_element _array_index) (Variables|Default|GetCurrentItems_P2)
    (if (== (.staticmesh_reference _array_element) (.staticmesh_reference (Variables|Default|GetDroppedItem_P2)))
      (return _array_index))))

(fn FindInitialParentItemEmpty
  (params (Input_Item :type STRUCT%20Items%20Structure))
  (bind _array_element (Utilities|Array|ForEachLoopwithBreak (Variables|Default|GetDT_Array))
    (:LoopBody
      (bind _returnvalue (Utilities|GetDataTableRow "/Game/Structs/DT_Items.DT_Items" _array_element)
        (:then
          (if (Utilities|Enum|Equal(Enum) (.object_name _returnvalue) (.parent_object Input_Item))
            (bind _itemindex (CallFunction|FindDroppedItemIndexinCurrentItemsP1))
            (return _array_element _itemindex (.object_name _returnvalue))))))))

(fn CreateListOfDesiredItems
  (bind _dt_array (Variables|Default|GetDT_Array))
  (Utilities|Array|Clear (Variables|Default|GetDesiredItems))
  (for (_array_element _array_index) (Variables|Default|GetCurrentItems_P1)
    (bind _elementtorespawn (CallFunction|FindInitialParentItemEmpty _array_element))
    (bind _returnvalue (Utilities|GetDataTableRow "/Game/Structs/DT_Items.DT_Items" (Utilities|Array|Get(acopy) (Variables|Default|GetDT_Array) (Math|Integer|Clamp(Integer) (+ (Utilities|Array|FindItem _dt_array _elementtorespawn) (Math|Random|RandomInteger (Math|Integer|Clamp(Integer) 1 1 2))) 0 (Utilities|Array|Length _dt_array))))
      (:then
        (Utilities|Array|SetArrayElem (Variables|Default|GetDesiredItems) _array_index _returnvalue)))))