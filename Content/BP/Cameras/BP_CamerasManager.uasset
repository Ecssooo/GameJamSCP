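; Camera manager for two local players that blends each player's view between a main camera and a hand camera.
; Per-player custom events call SetViewTargetWithBlend on player controllers 0 and 1 with configurable blend times, and combined events switch both players at once.
; BeginPlay runs a timed sequence that blends only player 1 to the hand camera, then back to the main camera.
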(event Custom|CE_InBlendCameraP1
  (bind _returnvalue (Game|GetPlayerController 0))
  ;[0.15 0.15 0.15 0.5] Camera blend Player 1
  (Utilities|IsValid _returnvalue
    (:Is%20Valid
      (Game|Player|SetViewTargetwithBlend _returnvalue (Variables|Player1|GetHandCameraP1) (Variables|Player1|GetInBlendTimeP1) "VTBlend_Linear" 1.0 false))))

(event Custom|CE_OutBlendCameraP1
  (bind _returnvalue (Game|GetPlayerController 0))
  ;[0.15 0.15 0.15 0.5] Camera blend Player 1
  (Utilities|IsValid _returnvalue
    (:Is%20Valid
      (Game|Player|SetViewTargetwithBlend _returnvalue (Variables|Player1|GetMainCameraP1) (Variables|Player1|GetOutBlendTimeP1) "VTBlend_Linear" 1.0 false))))

(event Custom|CE_InBlendCameraP2
  (bind _returnvalue (Game|GetPlayerController 1))
  ;[0.15 0.15 0.15 0.5] Camera blend player 2
  (Utilities|IsValid _returnvalue
    (:Is%20Valid
      (Game|Player|SetViewTargetwithBlend _returnvalue (Variables|Player2|GetHandCameraP2) (Variables|Player2|GetInBlendTimeP2) "VTBlend_Linear" 1.0 false))))

(event Custom|CE_OutBlendCameraP2
  (bind _returnvalue (Game|GetPlayerController 1))
  ;[0.15 0.15 0.15 0.5] Camera blend player 2
  (Utilities|IsValid _returnvalue
    (:Is%20Valid
      (Game|Player|SetViewTargetwithBlend _returnvalue (Variables|Player2|GetMainCameraP2) (Variables|Player2|GetOutBlendTimeP2) "VTBlend_Linear" 1.0 false))))

(event Custom|CE_InBlendAllCameras
  (CallFunction|CEinBlendCameraP1)
  (CallFunction|CEinBlendCameraP2))

(event Custom|CE_OutBlendAllCameras
  (CallFunction|CEOutBlendCameraP1)
  (CallFunction|CEOutBlendCameraP2))

(event EventBeginPlay
  (Utilities|FlowControl|Delay 1.0)
  (CallFunction|CEinBlendCameraP1)
  (Utilities|FlowControl|Delay 2.0)
  (CallFunction|CEOutBlendCameraP1))

(fn ConstructionScript)