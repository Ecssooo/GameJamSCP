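; Player-controlled hand that moves, tilts and grabs objects through Enhanced Input actions.
; HandMovement and HandRotation scale input by sensitivity and clamp it to ranges around the BeginPlay transform, with yaw set to zero.
; Box overlap stores actors implementing BPI_Object, and IA_Grab toggles their grabbed state through an interface message, passing the root component as parent.
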(event OnComponentBeginOverlap(Box)
  (params (OverlappedComponent :type Primitive%20Component%20Object%20Reference) (OtherActor :type Actor%20Object%20Reference) (OtherComp :type Primitive%20Component%20Object%20Reference) (OtherBodyIndex :type Integer) (bFromSweep :type Boolean) (SweepResult :type Hit%20Result%20Structure%20%28by%20ref%29))
  (if (Utilities|DoesObjectImplementInterface OtherActor "/Game/BP/Interface/BPI_Object.BPI_Object_C")
    (Variables|Default|SetObjectToInteract OtherActor)
    (Development|PrintString "In")))

(event OnComponentEndOverlap(Box)
  (params (OverlappedComponent :type Primitive%20Component%20Object%20Reference) (OtherActor :type Actor%20Object%20Reference) (OtherComp :type Primitive%20Component%20Object%20Reference) (OtherBodyIndex :type Integer))
  (if (Utilities|DoesObjectImplementInterface OtherActor "/Game/BP/Interface/BPI_Object.BPI_Object_C")
    (Variables|Default|SetObjectToInteract 0)
    (Development|PrintString "Out")))

(event Input|EnhancedActionEvents|EnhancedInputActionIA_Grab
  (params (ActionValue :type Boolean) (ElapsedSeconds :type Float%20%28double-precision%29) (TriggeredSeconds :type Float%20%28double-precision%29) (InputAction :type Input%20Action%20Object%20Reference :default "/Game/Inputs/Input/IA_Grab.IA_Grab"))
  (bind _defaultsceneroot (Variables|Default|GetDefaultSceneRoot))
  (:Started
    (Variables|Default|GetObjectToInteract
      (:then
        (if (Variables|Grab|Private|GetCanGrab)
          (if (Variables|Grab|Private|GetIsGrabbing)
            (Class|BPIObject|GetGrabbed(Message) (Variables|Default|GetObjectToInteract) true _defaultsceneroot)
            (Variables|Grab|Private|SetIsGrabbing false)
            (else
              (Class|BPIObject|GetGrabbed(Message) (Variables|Default|GetObjectToInteract) false _defaultsceneroot)
              (Variables|Grab|Private|SetIsGrabbing true)))))
      (:else))))

(event Input|EnhancedActionEvents|EnhancedInputActionIA_Move
  (params (ActionValue :type Vector :default "0, 0, 0") (ElapsedSeconds :type Float%20%28double-precision%29) (TriggeredSeconds :type Float%20%28double-precision%29) (InputAction :type Input%20Action%20Object%20Reference :default "/Game/Inputs/Input/IA_Move.IA_Move"))
  (CallFunction|HandMovement (.x ActionValue) (.y ActionValue) (.z ActionValue)))

(event Input|EnhancedActionEvents|EnhancedInputActionIA_Rotation
  (params (ActionValue :type Vector%202D%20Structure) (ElapsedSeconds :type Float%20%28double-precision%29) (TriggeredSeconds :type Float%20%28double-precision%29) (InputAction :type Input%20Action%20Object%20Reference :default "/Game/Inputs/Input/IA_Rotation.IA_Rotation"))
  (CallFunction|HandRotation (Math|Vector|MakeVector (.x ActionValue) (.y ActionValue) 0.0)))

(event EventBeginPlay
  (Variables|Movement|Private|SetHandMoveCenter (+ (Transformation|GetActorLocation) (Variables|Movement|GetMoveCenterOffset)))
  (Variables|Rotation|Private|SetRotationCenter (Transformation|GetActorRotation)))

(fn ConstructionScript)

(fn HandMovement
  (params (X :type Float%20%28double-precision%29) (Y :type Float%20%28double-precision%29) (Z :type Float%20%28double-precision%29))
  (bind _returnvalue (Transformation|GetActorLocation))
  (bind (_max _min) (Utilities|ClampRange))
  (bind _hand_move_sensi (Variables|Movement|GetHand%20Move%20Sensi))
  (bind (_x _y _z) (Math|Vector|BreakVector _min))
  (bind (_x_2 _y_2 _z_2) (Math|Vector|BreakVector _max))
  (bind (_x_out _y_out _z_out) (Utilities|ApplySensi X Y Z _hand_move_sensi))
  (Transformation|SetActorLocation (Math|Vector|MakeVector (Math|Float|Clamp(Float) (+ _x_out (.x _returnvalue)) _x _x_2) (Math|Float|Clamp(Float) (+ _y_out (.y _returnvalue)) _y _y_2) (Math|Float|Clamp(Float) (+ _z_out (.z _returnvalue)) _z _z_2)) false false))

(fn HandRotation
  (params (Input :type Vector))
  (bind (_max _min) (Utilities|ClampRotation))
  (bind _rotationsensi (Variables|Rotation|GetRotationSensi))
  (bind (_x_out _y_out) (Utilities|ApplySensi (.x Input) (.y Input) 0.0 _rotationsensi))
  (bind _output_get (Variables|Rotation|Private|SetRotationCurrent (Math|Rotator|MakeRotator (Math|Float|Clamp(Float) (+ (.roll (Variables|Rotation|Private|GetRotationCurrent)) _x_out) (.x _min) (.x _max)) (Math|Float|Clamp(Float) (+ (.pitch (Variables|Rotation|Private|GetRotationCurrent)) _y_out) (.y _min) (.y _max)) 0.0)))
  (Transformation|SetActorRotation _output_get))