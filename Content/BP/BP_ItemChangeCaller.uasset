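; BP_ItemChangeCaller is a trigger actor that asks BP_ItemManager to swap an overlapping item for a fine or rough version.
; FineCaller and RoughCaller overlaps filter for BPI_Object, read the player index and send the grabbed message.
; Each passes the overlapping static mesh to the manager, sets WantToMakeFine and calls FindItemToSpawn.
; The fine path also calls FindItemToSpawn once before identifying the mesh.
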(event Custom|OnComponentBeginOverlap_FINE
  (params (OverlappedComponent :type Primitive%20Component%20Object%20Reference) (OtherActor :type Actor%20Object%20Reference) (OtherComp :type Primitive%20Component%20Object%20Reference) (OtherBodyIndex :type Integer) (bFromSweep :type Boolean) (SweepResult :type Hit%20Result%20Structure%20%28by%20ref%29))
  (if (Utilities|DoesObjectImplementInterface OtherActor "/Game/BP/Interface/BPI_Object.BPI_Object_C")
    (bind _playerindex (Class|BPIObject|GetPlayerIndex(Message) OtherActor))
    (Class|BPIObject|GetGrabbed(Message) OtherActor true)
    (Default|FindItemtoSpawn (Variables|Default|GetBP_ItemManager_Ref) _playerindex)
    (bind _asstatic_mesh_component (Utilities|Casting|CastToStaticMeshComponent OtherComp))
    (Default|WhatItemIsThis? (Variables|Default|GetBP_ItemManager_Ref) _asstatic_mesh_component)
    (Variables|/Game/BP/BP_ItemManager.BP_ItemManager_C|SetWantToMakeFine? (Variables|Default|GetBP_ItemManager_Ref) true)
    (Default|FindItemtoSpawn (Variables|Default|GetBP_ItemManager_Ref) _playerindex)))

(event Custom|OnComponentBeginOverlap_ROUGH
  (params (OverlappedComponent :type Primitive%20Component%20Object%20Reference) (OtherActor :type Actor%20Object%20Reference) (OtherComp :type Primitive%20Component%20Object%20Reference) (OtherBodyIndex :type Integer) (bFromSweep :type Boolean) (SweepResult :type Hit%20Result%20Structure%20%28by%20ref%29))
  (if (Utilities|DoesObjectImplementInterface OtherActor "/Game/BP/Interface/BPI_Object.BPI_Object_C")
    (bind _playerindex (Class|BPIObject|GetPlayerIndex(Message) OtherActor))
    (Class|BPIObject|GetGrabbed(Message) OtherActor true)
    (bind _asstatic_mesh_component (Utilities|Casting|CastToStaticMeshComponent OtherComp))
    (Default|WhatItemIsThis? (Variables|Default|GetBP_ItemManager_Ref) _asstatic_mesh_component)
    (Variables|/Game/BP/BP_ItemManager.BP_ItemManager_C|SetWantToMakeFine? (Variables|Default|GetBP_ItemManager_Ref) false)
    (Default|FindItemtoSpawn (Variables|Default|GetBP_ItemManager_Ref) _playerindex)))

(event EventBeginPlay
  (bind _returnvalue (Actor|GetActorOfClass "/Game/BP/BP_ItemManager.BP_ItemManager_C"))
  (Variables|Default|SetBP_ItemManager_Ref _returnvalue)
  (Collision|AssignOnComponentBeginOverlap (Variables|Default|GetFineCaller) (delegate Custom|OnComponentBeginOverlap_FINE))
  (Collision|AssignOnComponentBeginOverlap (Variables|Default|GetRoughCaller) (delegate Custom|OnComponentBeginOverlap_ROUGH)))

(fn ConstructionScript)