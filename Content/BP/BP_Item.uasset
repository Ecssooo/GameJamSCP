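; BP_Item is an item actor whose static mesh switches between free physics and attachment through a GetGrabbed event.
; When IsGrabbed is true, it simulates physics with the PhysicsActor profile and detaches, despite the parameter's name.
; When false, it stops simulating, switches to BlockAllDynamic and attaches to the supplied Parent, keeping world transforms.
; Each branch prints On or Off as debug output.
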(event EventGetGrabbed
  (params (IsGrabbed :type Boolean) (Parent :type Scene%20Component%20Object%20Reference))
  (Physics|SetSimulatePhysics (Variables|Default|GetStaticMesh) IsGrabbed)
  (if IsGrabbed
    (Collision|SetCollisionProfileName (Variables|Default|GetStaticMesh) "PhysicsActor" true :!class /Script/Engine.PrimitiveComponent)
    (Development|PrintString "On")
    (Transformation|DetachFromActor "KeepWorld" "KeepWorld" "KeepWorld")
    (else
      (Collision|SetCollisionProfileName (Variables|Default|GetStaticMesh) "BlockAllDynamic" true :!class /Script/Engine.PrimitiveComponent)
      (Development|PrintString "Off")
      (Transformation|AttachComponentToComponent Parent "None" "KeepWorld" "KeepWorld" "KeepWorld" true))))

(fn ConstructionScript)