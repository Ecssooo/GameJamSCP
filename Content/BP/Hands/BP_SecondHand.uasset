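; BP_SecondHand is a hand actor with four fingers under a guillotine that cuts off the finger indexed by a passed-in score.
; The Drop timeline lowers the blade, then plays a sound, destroys that finger and unpauses a blood fountain particle system for one second.
; Separate events reverse the drop or run the Up timeline to raise the blade, with both timelines lerping from the blade's current location.
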(event Custom|CE_CutFinger
  (params (Score :type Integer))
  (bind _g_bot (Variables|Default|GetG_Bot))
  (bind _guillotine_lame (Variables|Default|GetGuillotine_lame))
  (bind _relativelocation (Variables|/Script/Engine.SceneComponent|GetRelativeLocation _guillotine_lame))
  ;[0.15 0.15 0.15 0.5] Guillotine Drop
  (bind (_direction _newtrack_0) (Timeline|Drop PlayFromStart)
    (:Update
      (Transformation|SetRelativeLocation (Variables|Default|GetGuillotine_lame) (Math|Vector|MakeVector (Math|Float|Lerp (.x _relativelocation) (.x _g_bot) _newtrack_0) (Math|Float|Lerp (.y _relativelocation) (.y _g_bot) _newtrack_0) (Math|Float|Lerp (.z _relativelocation) (.z _g_bot) _newtrack_0)) false false))
    (:Finished
      (Audio|PlaySoundatLocation "/Game/Audio/SFX/SFX_Second_Finger.SFX_Second_Finger" (Variables|/Script/Engine.SceneComponent|GetRelativeLocation (Variables|Default|GetCube)) "0, 0, 0" 1.0 1.0 -1.0 0 0 0 0)
      (switch Utilities|FlowControl|Switch|SwitchonETimelineDirection _direction
        (:Forward
          (Components|DestroyComponent (Utilities|Array|Get(acopy) (Variables|Default|GetFingersList) Score))
          (Class|NiagaraComponent|SetPaused (Variables|Default|GetPS_BloodFountain) false)
          (Utilities|FlowControl|Delay 1.0)
          (Class|NiagaraComponent|SetPaused (Variables|Default|GetPS_BloodFountain) true))))))

(event Custom|CE_RevertGuillotine
  (bind _g_bot (Variables|Default|GetG_Bot))
  (bind _guillotine_lame (Variables|Default|GetGuillotine_lame))
  (bind _relativelocation (Variables|/Script/Engine.SceneComponent|GetRelativeLocation _guillotine_lame))
  ;[0.15 0.15 0.15 0.5] Guillotine Drop
  (bind (_direction _newtrack_0) (Timeline|Drop ReverseFromEnd)
    (:Update
      (Transformation|SetRelativeLocation (Variables|Default|GetGuillotine_lame) (Math|Vector|MakeVector (Math|Float|Lerp (.x _relativelocation) (.x _g_bot) _newtrack_0) (Math|Float|Lerp (.y _relativelocation) (.y _g_bot) _newtrack_0) (Math|Float|Lerp (.z _relativelocation) (.z _g_bot) _newtrack_0)) false false))
    (:Finished
      (Audio|PlaySoundatLocation "/Game/Audio/SFX/SFX_Second_Finger.SFX_Second_Finger" (Variables|/Script/Engine.SceneComponent|GetRelativeLocation (Variables|Default|GetCube)) "0, 0, 0" 1.0 1.0 -1.0 0 0 0 0)
      (switch Utilities|FlowControl|Switch|SwitchonETimelineDirection _direction
        (:Forward
          (Components|DestroyComponent (Utilities|Array|Get(acopy) (Variables|Default|GetFingersList) (stale Custom|CE_CutFinger Score)))
          (Class|NiagaraComponent|SetPaused (Variables|Default|GetPS_BloodFountain) false)
          (Utilities|FlowControl|Delay 1.0)
          (Class|NiagaraComponent|SetPaused (Variables|Default|GetPS_BloodFountain) true))))))

(event Custom|CE_LameUp
  (bind _g_top (Variables|Default|GetG_Top))
  (bind _guillotine_lame (Variables|Default|GetGuillotine_lame))
  (bind _relativelocation (Variables|/Script/Engine.SceneComponent|GetRelativeLocation _guillotine_lame))
  (bind _newtrack_0 (Timeline|Up PlayFromStart)
    (:Update
      (Transformation|SetRelativeLocation (Variables|Default|GetGuillotine_lame) (Math|Vector|MakeVector (Math|Float|Lerp (.x _relativelocation) (.x _g_top) _newtrack_0) (Math|Float|Lerp (.y _relativelocation) (.y _g_top) _newtrack_0) (Math|Float|Lerp (.z _relativelocation) (.z _g_top) _newtrack_0)) false false))))

(event EventBeginPlay
  (Utilities|Array|Add (Variables|Default|GetFingersList) (Variables|Default|GetFinger1))
  (Utilities|Array|Add (Variables|Default|GetFingersList) (Variables|Default|GetFinger2))
  (Utilities|Array|Add (Variables|Default|GetFingersList) (Variables|Default|GetFinger3))
  (Utilities|Array|Add (Variables|Default|GetFingersList) (Variables|Default|GetFinger4))
  (bind _asgi_main (Utilities|Casting|CastToGI_Main (Game|GetGameInstance)))
  (Variables|Default|SetGameInstance _asgi_main)
  (Class|NiagaraComponent|SetPaused (Variables|Default|GetPS_BloodFountain) true))

(fn ConstructionScript)